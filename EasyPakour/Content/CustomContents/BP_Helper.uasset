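; BP_Helper is a set of stateless math helpers for offsetting positions and converting normals.
; Up and down moves shift a vector along world Z by a given amount.
; Forward, backward, right and left moves shift it along axes derived from a supplied rotation.
; ReverseNormal returns a rotator rather than a vector, built from the normal as X axis and offset by 180 degrees on one axis.
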(fn MoveVectorUpward
  (params (InVector :type Vector) (AddValue :type Float%20%28double-precision%29))
  (return (+ InVector (Math|Vector|MakeVector 0.0 0.0 AddValue))))

(fn MoveVectorDownward
  (params (InVector :type Vector) (SubstractValue :type Float%20%28double-precision%29))
  (return (- InVector (Math|Vector|MakeVector 0.0 0.0 SubstractValue))))

(fn MoveVectorForward
  (params (InVector :type Vector) (InRotation :type Rotator) (AddValue :type Float%20%28double-precision%29))
  (return (+ InVector (* (Math|Vector|GetForwardVector InRotation) AddValue))))

(fn MoveVectorBackward
  (params (InVector :type Vector) (InRotation :type Rotator) (SubstractValue :type Float%20%28double-precision%29))
  (return (- InVector (* (Math|Vector|GetForwardVector InRotation) SubstractValue))))

(fn MoveVectorRight
  (params (InVector :type Vector) (InRotator :type Rotator) (AddValue :type Float%20%28double-precision%29))
  (return (+ InVector (* (Math|Vector|GetRightVector InRotator) AddValue))))

(fn MoveVectorLeft
  (params (InVector :type Vector) (InRoattor :type Rotator) (SubstractValue :type Float%20%28double-precision%29))
  (return (- InVector (* (Math|Vector|GetRightVector InRoattor) SubstractValue))))

(fn ReverseNormal
  (params (InNormal :type Vector))
  (return (Math|Rotator|Delta(Rotator) (Math|Rotator|MakeRotfromX InNormal) "0.000000,180.000000,0.000000")))